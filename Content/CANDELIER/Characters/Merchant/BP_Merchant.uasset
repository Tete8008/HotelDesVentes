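; Merchant that offers one randomly chosen item and lets the player buy while in range.
; On BeginPlay it picks a random row from ItemsTable, relying on rows named by 1-based numbers, and stores it as SelectedItem.
; Capsule begin and end overlaps toggle CanBuy on the player's BP_Character, without checking which actor overlapped.
; The purchase itself is not handled here.
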(event `self.ReceiveBeginPlay`
  (bind _outrownames (`DataTableFunctionLibrary.GetDataTableRowNames` "/Game/CANDELIER/Blueprints/SaveGame/ItemsTable.ItemsTable"))
  (`self.PresentItem` (`KismetMathLibrary.RandomIntegerInRange` 1 (`KismetArrayLibrary.Array_Length` _outrownames))))

(event `PresentItem`
  (params (Index :type Integer))
  (bind _returnvalue (`|GetDataTableRow` "/Game/CANDELIER/Blueprints/SaveGame/ItemsTable.ItemsTable" (`KismetStringLibrary.Conv_StringToName` (`KismetStringLibrary.Conv_IntToString` Index)))
    (:`then`
      (set `self.SelectedItem` _returnvalue))))

(event `self.Capsule.OnComponentBeginOverlap`
  (params (OverlappedComponent :type "PrimitiveComponent Object Reference") (OtherActor :type "Actor Object Reference") (OtherComp :type "PrimitiveComponent Object Reference") (OtherBodyIndex :type Integer) (bFromSweep :type Boolean) (SweepResult :type "HitResult Structure (by ref)"))
  (set `/Game/CANDELIER/Characters/Mc_cree/BP_Character.CanBuy` true (cast `/Game/CANDELIER/Characters/Mc_cree/BP_Character` (`GameplayStatics.GetPlayerCharacter` 0) :!pure true)))

(event `self.Capsule.OnComponentEndOverlap`
  (params (OverlappedComponent :type "PrimitiveComponent Object Reference") (OtherActor :type "Actor Object Reference") (OtherComp :type "PrimitiveComponent Object Reference") (OtherBodyIndex :type Integer))
  (set `/Game/CANDELIER/Characters/Mc_cree/BP_Character.CanBuy` false (cast `/Game/CANDELIER/Characters/Mc_cree/BP_Character` (`GameplayStatics.GetPlayerCharacter` 0) :!pure true)))

(fn `UserConstructionScript`)